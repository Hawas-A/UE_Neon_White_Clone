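; Enemy pawn that chases the player and takes damage through a damage system component.
; On BeginPlay it moves toward the player with AI MoveTo, repeating after a short delay on success or immediately on failure.
; Health, heal and damage functions forward to BPCDamageSystem, whose death and damage-response events are bound in the construction script.
; Death ragdolls the mesh and sets a short lifespan, while damage responses are only printed.
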(event `self.ReceiveBeginPlay`
  ; Follow Player
  (`self.Chase Target` (`GameplayStatics.GetPlayerPawn` 0)))

(event `Chase Target`
  (params (TargetActor :type "Actor Object Reference"))
  ; Follow Player
  (`|AIMoveTo` self (0.0 0.0 0.0) TargetActor 120.0
    (:`OnSuccess`
      (`KismetSystemLibrary.Delay` 0.8))
    (:`OnFail`
      _))
  (`self.Chase Target` TargetActor))

(event `Death`
  (bind _mesh (`self.Mesh`))
  (`PrimitiveComponent.SetSimulatePhysics` _mesh true)
  (`PrimitiveComponent.SetCollisionEnabled` _mesh "PhysicsOnly")
  (`self.SetLifeSpan` 1.0))

(event `DamageResponse`
  (params (DamageResponse :type "/Game/DamageSystem/E_DamageResponse Enum" :default "NewEnumerator0"))
  (`KismetSystemLibrary.PrintString` (`|GetEnumeratorNameAsString` DamageResponse)))

(fn `GetCurrentHealth`
  (returns (Health :type "Float (double-precision)"))
  (bind _health (message `/Game/DamageSystem/BP_Damageable.GetCurrentHealth` (`self.BPC_DamageSystem`)))
  (return _health))

(fn `GetMaxHealth`
  (returns (MaxHealth :type "Float (double-precision)"))
  (bind _maxhealth (message `/Game/DamageSystem/BP_Damageable.GetMaxHealth` (`self.BPC_DamageSystem`)))
  (return _maxhealth))

(fn `Heal`
  (params (HealAmount :type "Float (double-precision)"))
  (returns (NewHealth :type "Float (double-precision)"))
  (bind _newhealth (`/Game/DamageSystem/BPC_DamageSystem.Heal` (`self.BPC_DamageSystem`) HealAmount))
  (return _newhealth))

(fn `TakeDamage`
  (params (DamageInfo :type "/Game/DamageSystem/S_DamageInfo Structure"))
  (returns (WasDamaged :type Boolean))
  (bind _wasdamaged (`/Game/DamageSystem/BPC_DamageSystem.TakeDamage` (`self.BPC_DamageSystem`) DamageInfo))
  (return _wasdamaged))

(fn `UserConstructionScript`
  (bind _bpc_damagesystem (`self.BPC_DamageSystem`))
  (add `/Game/DamageSystem/BPC_DamageSystem.OnDeath` _bpc_damagesystem (`|CreateDelegate` :!event `Death`))
  (add `/Game/DamageSystem/BPC_DamageSystem.OnDamageResponse` _bpc_damagesystem (`|CreateDelegate` :!event `DamageResponse`)))